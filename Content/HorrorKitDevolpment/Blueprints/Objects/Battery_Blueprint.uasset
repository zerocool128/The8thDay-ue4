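; Battery pickup actor that adds a battery to the player's inventory when interacted with.
; The InteractableObject event casts the player character to Main_Character_Blueprint, increments its battery count clamped to the maximum, then destroys the actor.
; The pickup is destroyed even if the player is already at the maximum.
; The construction script applies the configurable BatteryMesh to the static mesh component.
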(event EventInteractableObject
  ;[1 1 1] Interactable Battery and how much they gain
  (bind _asmain_character_blueprint (Utilities|Casting|CastToMain_Character_Blueprint (Game|GetPlayerCharacter 0)))
  (Variables|/Game/HorrorKitDevolpment/Blueprints/Character/Main_Character_Blueprint.Main_Character_Blueprint_C|SetNumber%20of%20Batteries _asmain_character_blueprint (Math|Integer|Clamp(Integer) (+ (Variables|/Game/HorrorKitDevolpment/Blueprints/Character/Main_Character_Blueprint.Main_Character_Blueprint_C|GetNumber%20of%20Batteries _asmain_character_blueprint) 1) 0 (Variables|/Game/HorrorKitDevolpment/Blueprints/Character/Main_Character_Blueprint.Main_Character_Blueprint_C|GetMax%20Number%20of%20Batteries _asmain_character_blueprint)))
  (Actor|DestroyActor))

(fn ConstructionScript
  ;[1 1 1] Set new Mesh for Battery
  (Components|StaticMesh|SetStaticMesh (Variables|Default|GetStaticMesh) (Variables|HK:BatteryBlueprint|GetBattery%20Mesh)))