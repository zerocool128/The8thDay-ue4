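; Flickering, sparking ceiling lamp for the horror game, with a configurable point light.
; The construction script applies the brightness, color and source radius variables to the point light.
; Tick drives two Delays of different lengths that act as repeating timers, each toggling spark burst visibility and setting one of two lamp materials.
; The flicker affects only the sparks and lamp material, leaving the point light steady.
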(event EventTick
  (params (DeltaSeconds :type Float%20%28single-precision%29))
  (bind _sm_lamp_ceiling (Variables|Default|GetSM_Lamp_Ceiling))
  (Utilities|FlowControl|Sequence
    (:then_0
      (Utilities|FlowControl|Delay 0.2)
      (Rendering|ToggleVisibility (Variables|Default|GetP_spark_burst) false)
      (Rendering|Material|SetMaterial _sm_lamp_ceiling 0 "/Game/Hospital/Hospital_Pack/Structural/CeilingDecorative/Materials/MI_Hanging_Ceiling2.MI_Hanging_Ceiling2"))
    (:then_1
      (Utilities|FlowControl|Delay 0.5)
      (Rendering|ToggleVisibility (Variables|Default|GetP_spark_burst) false)
      (Rendering|Material|SetMaterial _sm_lamp_ceiling 0 "/Game/Hospital/Hospital_Pack/Structural/CeilingDecorative/Materials/MI_Hanging_Ceiling.MI_Hanging_Ceiling"))))

(fn ConstructionScript
  (bind _pointlight1 (Variables|Default|GetPointLight1))
  (Utilities|FlowControl|Sequence
    (:then_0
      (Rendering|Components|Light|SetIntensity _pointlight1 (Variables|Light|GetBrightness))
      (Rendering|Components|Light|SetLightColor _pointlight1 (Variables|Light|GetColor_0) true)
      (Class|PointLightComponent|SetSourceRadius _pointlight1 (Variables|Light|GetSource%20Radius)))))