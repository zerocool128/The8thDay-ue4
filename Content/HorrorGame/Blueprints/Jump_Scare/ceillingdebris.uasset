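; Ceiling debris jump scare actor that drops debris meshes and shakes the camera after a box trigger is overlapped.
; On any overlap, it turns physics off on six static meshes, waits five seconds, then toggles their visibility and enables physics simulation.
; It then plays a world camera shake oriented toward a hardcoded epicenter, with no actor filter or one-shot guard on the trigger.
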(event OnComponentBeginOverlap(Box)
  (params (OverlappedComponent :type Primitive%20Component%20Object%20Reference) (OtherActor :type Actor%20Object%20Reference) (OtherComp :type Primitive%20Component%20Object%20Reference) (OtherBodyIndex :type Integer) (bFromSweep :type Boolean) (SweepResult :type Hit%20Result%20Structure%20%28by%20ref%29))
  (bind _staticmesh1 (Variables|Default|GetStaticMesh1))
  (Physics|SetSimulatePhysics _staticmesh1 false)
  (Utilities|FlowControl|Delay 5.0)
  (Rendering|ToggleVisibility _staticmesh1 false)
  (Physics|SetSimulatePhysics _staticmesh1 true)
  (Camera|PlayWorldCameraShake "/Script/Engine.CameraShake" "500.000000,500.000000,500.000000" 0.0 0.0 1.0 true))

(fn ConstructionScript)