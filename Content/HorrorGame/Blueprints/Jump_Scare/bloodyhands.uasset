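; Horror jump scare Blueprint, named for bloody hands, that fires the first time any actor overlaps it.
; A do-once gate starts a short delay, then plays a scare sound at the world origin.
; A sequence of parallel, increasing delays then toggles the visibility of eight decal components one after another, creating a staggered effect.
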(event Collision|EventActorBeginOverlap
  (params (OtherActor :type Actor%20Object%20Reference))
  (|DoOnceMultiInput
    (:A%20Out
      (Utilities|FlowControl|Delay 1.0)
      (Audio|PlaySoundatLocation "/Game/Audio/Jump_Scare_01.Jump_Scare_01" "0, 0, 0")
      (Utilities|FlowControl|Sequence
        (:then_0
          (Utilities|FlowControl|Delay 0.2)
          (Rendering|ToggleVisibility (Variables|Default|GetDecal) false))
        (:then_1
          (Utilities|FlowControl|Delay 0.4)
          (Rendering|ToggleVisibility (Variables|Default|GetDecal1) false))
        (:then_2
          (Utilities|FlowControl|Delay 0.6)
          (Rendering|ToggleVisibility (Variables|Default|GetDecal2) false))
        (:then_3
          (Utilities|FlowControl|Delay 0.8)
          (Rendering|ToggleVisibility (Variables|Default|GetDecal3) false))
        (:then_4
          (Utilities|FlowControl|Delay 0.9)
          (Rendering|ToggleVisibility (Variables|Default|GetDecal4) false))
        (:then_5
          (Utilities|FlowControl|Delay 1.0)
          (Rendering|ToggleVisibility (Variables|Default|GetDecal5) false))
        (:then_6
          (Utilities|FlowControl|Delay 1.2)
          (Rendering|ToggleVisibility (Variables|Default|GetDecal6) false))
        (:then_7
          (Utilities|FlowControl|Delay 1.3)
          (Rendering|ToggleVisibility (Variables|Default|GetDecal7) false))))))

(fn ConstructionScript)