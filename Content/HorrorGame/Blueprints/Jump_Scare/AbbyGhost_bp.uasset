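; AbbyGhost_bp is a one-shot jump-scare trigger that flashes Abby ghost widgets on screen when its box is overlapped.
; A Sequence checks boolean flags for three ghost variants and a camera shake, so enabled branches run concurrently.
; Two variants play a sound, wait, briefly show their widget, then play another; the third shows its widget immediately, without sound.
; Sounds play at world origin, and the shake uses a fixed world epicenter.
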(event OnComponentBeginOverlap(Triggerboxabby)
  (params (OverlappedComponent :type Primitive%20Component%20Object%20Reference) (OtherActor :type Actor%20Object%20Reference) (OtherComp :type Primitive%20Component%20Object%20Reference) (OtherBodyIndex :type Integer) (bFromSweep :type Boolean) (SweepResult :type Hit%20Result%20Structure%20%28by%20ref%29))
  (|DoOnceMultiInput
    (:A%20Out
      (Utilities|FlowControl|Sequence
        (:then_0
          (if (Variables|Default|Getplay%20ghos3)
            (Audio|PlaySoundatLocation (Variables|Default|GetSound%20Asset) "0, 0, 0")
            (Utilities|FlowControl|Delay 3.0)
            (bind _returnvalue (UserInterface|CreateWidget "/Game/HorrorGame/Abbyghost.Abbyghost_C"))
            (UserInterface|Viewport|AddtoViewport _returnvalue 0)
            (Utilities|FlowControl|Delay 1.0)
            (Widget|RemovefromParent _returnvalue)
            (Audio|PlaySoundatLocation (Variables|Default|GetSound%20Asset2) "0, 0, 0")))
        (:then_1
          (if (Variables|Default|Getplay%20ghost1)
            (Audio|PlaySoundatLocation (Variables|Default|GetSound%20Asset) "0, 0, 0")
            (Utilities|FlowControl|Delay 3.0)
            (bind _returnvalue_2 (UserInterface|CreateWidget "/Game/HorrorGame/Abbyghost3.Abbyghost3_C"))
            (UserInterface|Viewport|AddtoViewport _returnvalue_2 0)
            (Utilities|FlowControl|Delay 1.0)
            (Widget|RemovefromParent _returnvalue_2)
            (Audio|PlaySoundatLocation (Variables|Default|GetSound%20Asset3) "0, 0, 0")))
        (:then_2
          (if (Variables|Default|Getplay%20ghost2)
            (bind _returnvalue_3 (UserInterface|CreateWidget "/Game/HorrorGame/Abbyghost2.Abbyghost2_C"))
            (UserInterface|Viewport|AddtoViewport _returnvalue_3 0)
            (Utilities|FlowControl|Delay 1.0)
            (Widget|RemovefromParent _returnvalue_3)))
        (:then_3
          (if (Variables|Default|GetCamerashake)
            (Camera|PlayWorldCameraShake "/Script/Engine.CameraShake" "45.000000,45.000000,45.000000" 1e+02 3e+02 25.0 true)))))))

(fn ConstructionScript)