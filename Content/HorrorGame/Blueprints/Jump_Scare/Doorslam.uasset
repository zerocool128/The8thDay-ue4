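; Horror jump-scare door that slams once when an actor overlaps it, then destroys itself after a delay.
; The overlap plays an explosion sound, rotates the door mesh with an eased MoveComponentTo, and follows with a delayed voice-line sound.
; A separate Boxdoorlocked trigger enables player input and opens a gate, so pressing Interact inside it plays a locked-door sound.
; All sounds play at world origin.
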(event OnComponentBeginOverlap(Boxdoorlocked)
  (params (OverlappedComponent :type Primitive%20Component%20Object%20Reference) (OtherActor :type Actor%20Object%20Reference) (OtherComp :type Primitive%20Component%20Object%20Reference) (OtherBodyIndex :type Integer) (bFromSweep :type Boolean) (SweepResult :type Hit%20Result%20Structure%20%28by%20ref%29))
  ;[1 1 1] Door Locked sound
  (Input|EnableInput (Game|GetPlayerController 0))
  (Utilities|FlowControl|Gate true) ; enters at Open
)

(event OnComponentEndOverlap(Boxdoorlocked)
  (params (OverlappedComponent :type Primitive%20Component%20Object%20Reference) (OtherActor :type Actor%20Object%20Reference) (OtherComp :type Primitive%20Component%20Object%20Reference) (OtherBodyIndex :type Integer))
  ;[1 1 1] Door Locked sound
  (Input|DisableInput (Game|GetPlayerController 0))
  (Utilities|FlowControl|Gate true) ; enters at Close
)

(event Collision|EventActorBeginOverlap
  (params (OtherActor :type Actor%20Object%20Reference))
  (bind _sm_door_01 (Variables|Default|GetSM_Door_01))
  (|DoOnceMultiInput
    (:A%20Out
      (Audio|PlaySoundatLocation "/Game/Audio/Explosion01.Explosion01" "0, 0, 0")
      ;[1 1 1] Rotate Door
      (Utilities|FlowControl|Sequence
        (:then_0
          (Utilities|FlowControl|Delay 0.2)
          (Components|MoveComponentTo _sm_door_01 (Variables|/Script/Engine.SceneComponent|GetRelativeLocation _sm_door_01) (Variables|Default|Getrotdoor) true true (Variables|Default|Getdoorspeed) false)
          (Utilities|FlowControl|Delay 3e+01)
          (Actor|DestroyActor))
        (:then_1
          (Utilities|FlowControl|Delay 2.0)
          (Audio|PlaySoundatLocation "/Game/Audio/Actorvoice/Ohgod.Ohgod" "0, 0, 0"))))))

(event Input|ActionEvents|InputActionInteract
  (params (Key :type Key%20Structure :default "AnyKey"))
  ;[1 1 1] Door Locked sound
  (:Pressed
    (Utilities|FlowControl|Gate true
      (:Exit
        (Audio|PlaySoundatLocation "/Game/Audio/Sounds/Audio/lockeddoor2.lockeddoor2" "0, 0, 0")))))

(fn ConstructionScript)