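; Elevator actor in a horror game that slides its static mesh between two positions when the player presses Interact inside a trigger box.
; Two box overlaps enable input and open separate gates, so one plays the movement timeline and the other reverses it.
; The timeline lerps the mesh's relative location between Drawerstart and Drawerend, firing the creepy elevator sound at world origin on every update.
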(event OnComponentBeginOverlap(Box)
  (params (OverlappedComponent :type Primitive%20Component%20Object%20Reference) (OtherActor :type Actor%20Object%20Reference) (OtherComp :type Primitive%20Component%20Object%20Reference) (OtherBodyIndex :type Integer) (bFromSweep :type Boolean) (SweepResult :type Hit%20Result%20Structure%20%28by%20ref%29))
  (Input|EnableInput (Game|GetPlayerController 0))
  (Utilities|FlowControl|Gate true) ; enters at Open
)

(event OnComponentEndOverlap(Box)
  (params (OverlappedComponent :type Primitive%20Component%20Object%20Reference) (OtherActor :type Actor%20Object%20Reference) (OtherComp :type Primitive%20Component%20Object%20Reference) (OtherBodyIndex :type Integer))
  (Input|DisableInput (Game|GetPlayerController 0))
  (Utilities|FlowControl|Gate true) ; enters at Close
)

(event OnComponentBeginOverlap(Box1)
  (params (OverlappedComponent :type Primitive%20Component%20Object%20Reference) (OtherActor :type Actor%20Object%20Reference) (OtherComp :type Primitive%20Component%20Object%20Reference) (OtherBodyIndex :type Integer) (bFromSweep :type Boolean) (SweepResult :type Hit%20Result%20Structure%20%28by%20ref%29))
  (Input|EnableInput (Game|GetPlayerController 0))
  (Utilities|FlowControl|Gate true) ; enters at Open
)

(event OnComponentEndOverlap(Box1)
  (params (OverlappedComponent :type Primitive%20Component%20Object%20Reference) (OtherActor :type Actor%20Object%20Reference) (OtherComp :type Primitive%20Component%20Object%20Reference) (OtherBodyIndex :type Integer))
  (Input|DisableInput (Game|GetPlayerController 0))
  (Utilities|FlowControl|Gate true) ; enters at Close
)

(event Input|ActionEvents|InputActionInteract
  (params (Key :type Key%20Structure :default "AnyKey"))
  (:Pressed
    (Utilities|FlowControl|Gate true
      (:Exit
        (bind _driver (Timeline|Timeline_0 Reverse)
          (:Update
            (Audio|PlaySoundatLocation "/Game/Audio/Sounds/Audio/creepyelevator.creepyelevator" "0, 0, 0")
            (Transformation|SetRelativeLocation (Variables|Default|GetStaticMesh) (Math|Vector|Lerp(Vector) (Variables|Default|GetDrawerstart) (Variables|Default|GetDrawerend) _driver) false false)))))))

(event Input|ActionEvents|InputActionInteract
  (params (Key :type Key%20Structure :default "AnyKey"))
  (:Pressed
    (Utilities|FlowControl|Gate true
      (:Exit
        (bind _driver (Timeline|Timeline_0 Play)
          (:Update
            (Audio|PlaySoundatLocation "/Game/Audio/Sounds/Audio/creepyelevator.creepyelevator" "0, 0, 0")
            (Transformation|SetRelativeLocation (Variables|Default|GetStaticMesh) (Math|Vector|Lerp(Vector) (Variables|Default|GetDrawerstart) (Variables|Default|GetDrawerend) _driver) false false)))))))

(fn ConstructionScript)