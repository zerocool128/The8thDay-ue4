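; Interactable text-display actor that toggles the Nothinguseful widget when Interact is pressed within its overlap area.
; Begin and end overlap enable or disable input for player controller 0 and open or close a gate on the Interact event, with no check on which actor overlaps.
; A FlipFlop alternates between showing the widget with cinematic mode locking movement and turning, and removing it to restore control.
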(event Collision|EventActorBeginOverlap
  (params (OtherActor :type Actor%20Object%20Reference))
  (bind _returnvalue (Game|GetPlayerController 0))
  (Input|EnableInput _returnvalue)
  (Utilities|FlowControl|Gate false) ; enters at Open
)

(event Collision|EventActorEndOverlap
  (params (OtherActor :type Actor%20Object%20Reference))
  (bind _returnvalue (Game|GetPlayerController 0))
  (Input|DisableInput _returnvalue)
  (Utilities|FlowControl|Gate false) ; enters at Close
)

(event Input|ActionEvents|InputActionInteract
  (params (Key :type Key%20Structure :default "AnyKey"))
  (bind _returnvalue (Game|GetPlayerController 0))
  (:Pressed
    (Utilities|FlowControl|Gate false
      (:Exit
        (Utilities|FlowControl|FlipFlop
          (:A
            (Class|PlayerController|SetCinematicMode _returnvalue true false true true true)
            (bind _returnvalue_2 (UserInterface|CreateWidget "/Game/HorrorGame/PickUps/Text_display/Nothing_useful/Nothinguseful.Nothinguseful_C" _returnvalue))
            (UserInterface|Viewport|AddtoViewport _returnvalue_2 0))
          (:B
            (Class|PlayerController|SetCinematicMode _returnvalue false false true true true)
            (Widget|RemovefromParent _returnvalue_2)))))))

(fn ConstructionScript)