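; Readable note pickup for the horror game that shows the Run_Not widget while the player is nearby.
; Actor overlap enables input and opens a gate, letting E or the top gamepad face button reach a FlipFlop.
; The first press enters cinematic mode, locking movement and turning, and displays the note.
; The second restores control, removes the widget and destroys the actor, so the note is single-use.
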(event Collision|EventActorBeginOverlap
  (params (OtherActor :type Actor%20Object%20Reference))
  (bind _returnvalue (Game|GetPlayerController 0))
  (Input|EnableInput _returnvalue)
  (Utilities|FlowControl|Gate false) ; enters at Open
)

(event Collision|EventActorEndOverlap
  (params (OtherActor :type Actor%20Object%20Reference))
  (bind _returnvalue (Game|GetPlayerController 0))
  (Input|DisableInput _returnvalue)
  (Utilities|FlowControl|Gate false) ; enters at Close
)

(event Input|GamepadEvents|GamepadFaceButtonTop
  (params (Key :type Key%20Structure :default "AnyKey"))
  (bind _returnvalue (Game|GetPlayerController 0))
  (:Pressed
    (Utilities|FlowControl|Gate false
      (:Exit
        (Utilities|FlowControl|FlipFlop
          (:A
            (Class|PlayerController|SetCinematicMode _returnvalue true true true true true)
            (bind _returnvalue_2 (UserInterface|CreateWidget "/Game/HorrorGame/PickUps/Notes/Run_Note/Run_Not.Run_Not_C" _returnvalue))
            (UserInterface|Viewport|AddtoViewport _returnvalue_2 0))
          (:B
            (Class|PlayerController|SetCinematicMode _returnvalue false false true true true)
            (Widget|RemovefromParent _returnvalue_2)
            (Actor|DestroyActor)))))))

(event Input|KeyboardEvents|E
  (params (Key :type Key%20Structure :default "AnyKey"))
  (bind _returnvalue (Game|GetPlayerController 0))
  (:Pressed
    (Utilities|FlowControl|Gate false
      (:Exit
        (Utilities|FlowControl|FlipFlop
          (:A
            (Class|PlayerController|SetCinematicMode _returnvalue true true true true true)
            (bind _returnvalue_2 (UserInterface|CreateWidget "/Game/HorrorGame/PickUps/Notes/Run_Note/Run_Not.Run_Not_C" _returnvalue))
            (UserInterface|Viewport|AddtoViewport _returnvalue_2 0))
          (:B
            (Class|PlayerController|SetCinematicMode _returnvalue false false true true true)
            (Widget|RemovefromParent _returnvalue_2)
            (Actor|DestroyActor)))))))

(fn ConstructionScript)